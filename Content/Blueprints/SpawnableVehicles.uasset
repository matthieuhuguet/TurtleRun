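; SpawnableVehicles is a character-based vehicle that travels by AI movement to an arrival point.
; Its construction script converts IntegerForCustomVehicles into a row name in DT_Vehicles, then applies that row's mesh and maximum walk speed, so one Blueprint covers several vehicle types.
; On BeginPlay, it issues an AI move to the world location of Arrivals.
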(event EventBeginPlay
  (AI|AIMoveTo self (Transformation|GetWorldLocation (Variables|Default|GetArrivals)) 0 5.0 false))

(event Collision|EventActorBeginOverlap
  (params (OtherActor :type Actor%20Object%20Reference)))

(event EventTick
  (params (DeltaSeconds :type Float%20%28single-precision%29)))

(fn ConstructionScript
  (bind _returnvalue (Utilities|GetDataTableRow "/Game/Blueprints/DT_Vehicles.DT_Vehicles" (Utilities|String|StringToName (Utilities|String|ToString(Integer) (Variables|Default|GetIntegerForCustomVehicles))))
    (:then
      (Components|StaticMesh|SetStaticMesh (Variables|Default|GetStaticMesh) (.MeshForVehicles (Utilities|Struct|BreakAll_Vehicles _returnvalue)))
      (Variables|/Script/Engine.CharacterMovementComponent|SetMaxWalkSpeed (Variables|Character|GetCharacterMovement) (.Speed (Utilities|Struct|BreakAll_Vehicles _returnvalue))))))