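; Spawnable turtle character that walks by AI to a destination when play begins.
; The construction script reads a fixed row from the deprecated turtle data table to set its static mesh and max walk speed.
; BeginPlay issues an AI MoveTo toward the world location of Arrivals, with zero acceptance radius.
; Overlap and Tick are disabled stubs, and Spawn is unused.
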(event EventBeginPlay
  (AI|AIMoveTo self (Transformation|GetWorldLocation (Variables|Default|GetArrivals)) 0 0.0 false))

(event Collision|EventActorBeginOverlap
  (params (OtherActor :type Actor%20Object%20Reference)))

(event EventTick
  (params (DeltaSeconds :type Float%20%28single-precision%29)))

(fn ConstructionScript
  (bind _returnvalue (Utilities|GetDataTableRow "/Game/Blueprints/Turtles/DT_TurtuleDeprecated.DT_TurtuleDeprecated" "NewRow")
    (:then
      (Components|StaticMesh|SetStaticMesh (Variables|Default|GetStaticMesh) (.MeshForTurtules (Utilities|Struct|BreakAll_Turtles _returnvalue)))
      (Variables|/Script/Engine.CharacterMovementComponent|SetMaxWalkSpeed (Variables|Character|GetCharacterMovement) (.Speed (Utilities|Struct|BreakAll_Turtles _returnvalue))))))