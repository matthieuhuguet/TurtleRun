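; SpawnableTurtles2 is a turtle character that mirrors the motion of a referenced FollowSpline object.
; Each Tick it copies that object's Distance and snaps its own location and rotation to the world transform of the spline's Cube component.
; Unconnected leftover logic would set the mesh and walk speed from the deprecated turtle data table, but it never runs.
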(event EventBeginPlay)

(event Collision|EventActorBeginOverlap
  (params (OtherActor :type Actor%20Object%20Reference)))

(event EventTick
  (params (DeltaSeconds :type Float%20%28single-precision%29))
  (bind _followspline (Variables|Default|GetFollowSpline))
  (bind _cube (Variables|/Game/Blueprints/Vehicules/BP_FollowSplineTurtle.BP_FollowSplineTurtle_C|GetCube _followspline))
  (bind _returnvalue (Transformation|GetWorldTransform _cube))
  (Variables|Default|SetDistance (Variables|/Game/Blueprints/Vehicules/BP_FollowSplineTurtle.BP_FollowSplineTurtle_C|GetDistance _followspline))
  (Transformation|SetActorTransform (Math|Transform|MakeTransform (.location _returnvalue) (.rotation _returnvalue) "1.000000,1.000000,1.000000")))

(fn ConstructionScript)