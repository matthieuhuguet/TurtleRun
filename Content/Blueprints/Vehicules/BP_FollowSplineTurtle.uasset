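; BP_FollowSplineTurtle is a vehicle Blueprint that moves its Cube component along its Spline.
; Each Tick raises Speed by delta time, so motion keeps accelerating, then advances Distance and sets the Cube's relative location and rotation from the spline in local space.
; When IsLooping is set, Distance resets to zero past the spline's end while Speed keeps growing.
; Disconnected array, timeline and switch nodes are unused.
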(event EventBeginPlay
  ;[1 0.375 0.6307] Another system
)

(event Collision|EventActorBeginOverlap
  (params (OtherActor :type Actor%20Object%20Reference))
  ;[1 0.375 0.6307] Another system
)

(event EventTick
  (params (DeltaSeconds :type Float%20%28single-precision%29))
  (Variables|Default|SetSpeed (+ DeltaSeconds (Variables|Default|GetSpeed)))
  (Variables|Default|SetDistance (+ (* DeltaSeconds (Variables|Default|GetSpeed)) (Variables|Default|GetDistance)))
  (Transformation|SetRelativeTransform (Variables|Default|GetCube) (Math|Transform|MakeTransform (.location (Spline|GetTransformatDistanceAlongSpline (Variables|Default|GetSpline) (Variables|Default|GetDistance) "Local" false)) (.rotation (Spline|GetTransformatDistanceAlongSpline (Variables|Default|GetSpline) (Variables|Default|GetDistance) "Local" false)) (Variables|/Script/Engine.SceneComponent|GetRelativeScale3D (Variables|Default|GetCube))) false false)
  (if (Variables|Default|GetIsLooping)
    (if (> (Variables|Default|GetDistance) (Spline|GetSplineLength (Variables|Default|GetSpline)))
      (Variables|Default|SetDistance 0.0))))

(fn ConstructionScript)