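; Tank is a clickable vehicle that copies the transform of a FollowSpline cube every tick.
; Turtles overlapping its hit box are destroyed after a short delay, and the player character takes damage, in logic marked deprecated.
; Hovering swaps the mesh material, and an actor click spawns an explosion and destroys it.
; A capsule click also destroys it once Counter reaches a threshold, but the increment is unwired and scoring only prints text.
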(event OnComponentBeginOverlap(CreateBoxForHit)
  (params (OverlappedComponent :type Primitive%20Component%20Object%20Reference) (OtherActor :type Actor%20Object%20Reference) (OtherComp :type Primitive%20Component%20Object%20Reference) (OtherBodyIndex :type Integer) (bFromSweep :type Boolean) (SweepResult :type Hit%20Result%20Structure%20%28by%20ref%29))
  (bind _asspawnable_turtles_2 (Utilities|Casting|CastToSpawnableTurtles2 OtherActor))
  (Utilities|FlowControl|Delay 0.016667)
  (Utilities|FlowControl|Sequence
    (:then_0
      ;[1 0.3229 0.5518] Deprecated Please do Optimise
      (bind _asbp_top_down_character_1 (Utilities|Casting|CastToBP_TopDownCharacter1 (Game|GetPlayerCharacter 0)))
      (Game|Damage|ApplyDamage _asbp_top_down_character_1 1.0 0 0))
    (:then_1
      (Actor|DestroyActor _asspawnable_turtles_2))))

(event OnClicked(CapsuleComponent)
  (params (TouchedComponent :type Primitive%20Component%20Object%20Reference) (ButtonPressed :type Key%20Structure))
  (if (>= (Variables|Default|GetCounter) (Variables|Default|GetIntegerForCustomVehicles))
    (Utilities|FlowControl|Sequence
      (:then_0
        (Development|PrintString "Add score"))
      (:then_1
        (Actor|DestroyActor self)))))

(event EventTick
  (params (DeltaSeconds :type Float%20%28single-precision%29))
  (bind _followspline (Variables|Default|GetFollowSpline))
  (bind _cube (Variables|/Game/Blueprints/Vehicules/BP_FollowSpline.BP_FollowSpline_C|GetCube _followspline))
  (bind _returnvalue (Transformation|GetWorldTransform _cube))
  (Variables|Default|SetDistance (Variables|/Game/Blueprints/Vehicules/BP_FollowSpline.BP_FollowSpline_C|GetDistance _followspline))
  (Transformation|SetActorTransform (Math|Transform|MakeTransform (.location _returnvalue) (.rotation _returnvalue) "1.000000,1.000000,1.000000")))

(event Collision|EventActorBeginOverlap
  (params (OtherActor :type Actor%20Object%20Reference)))

(event EventBeginPlay)

(event MouseInput|EventActorOnClicked
  (params (ButtonPressed :type Key%20Structure))
  (bind _staticmesh (Variables|Default|GetStaticMesh))
  (Effects|SpawnEmitteratLocation "/Game/StarterContent/Particles/P_Explosion.P_Explosion" (Transformation|GetWorldLocation _staticmesh) (Transformation|GetWorldRotation _staticmesh))
  (Actor|DestroyActor))

(event MouseInput|EventActorBeginCursorOver
  (Rendering|Material|SetMaterial (Variables|Default|GetStaticMesh) 0 "/Game/Cursor/M_Cursor.M_Cursor"))

(event MouseInput|EventActorEndCursorOver
  (Rendering|Material|SetMaterial (Variables|Default|GetStaticMesh) 0 "/Game/CrossyRoadAssets/blinn16.blinn16"))

(fn ConstructionScript)