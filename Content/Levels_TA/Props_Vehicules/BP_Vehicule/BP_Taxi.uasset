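; BP_Taxi is a taxi vehicle prop that fakes a driving motion through procedural animation.
; BeginPlay caches the body's relative transform, and Tick accumulates elapsed time to drive sine waves.
; These waves bob the body vertically by Jump and rock its roll by Balencement at half that frequency.
; The four wheels spin in pitch by TaxiSpeed each frame, without delta-time scaling.
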(event EventBeginPlay
  (bind _taxi (Variables|Default|GetTaxi))
  ;[0.5422 0.386 1] Position meshes
  (Variables|Default|SetRelative%20Location (Variables|/Script/Engine.SceneComponent|GetRelativeLocation _taxi))
  (Variables|Default|SetRelative%20Rotation (Variables|/Script/Engine.SceneComponent|GetRelativeRotation _taxi)))

(event Collision|EventActorBeginOverlap
  (params (OtherActor :type Actor%20Object%20Reference)))

(event EventTick
  (params (DeltaSeconds :type Float%20%28single-precision%29))
  (bind _jump (Variables|Default|Getjump))
  (bind _balencement (Variables|Default|Getbalencement))
  (bind _relative_location (Variables|Default|GetRelative%20Location))
  ;[1 0.3444 0.8431] Valeure de repetition
  (Variables|Default|SetNewVar_0 (+ DeltaSeconds (Variables|Default|GetNewVar_0)))
  ;[0.09375 0.6472 1] Rotation des roues
  (Transformation|AddLocalRotation (Variables|Default|GetRoue_Taxi) (Math|Rotator|MakeRotator 0.0 (Variables|Default|GetTaxiSpeed) 0.0) false false)
  (Transformation|SetRelativeLocationAndRotation (Variables|Default|GetTaxi) (Math|Vector|Lerp(Vector) (Math|Vector|MakeVector 0.0 0.0 (- (.z _relative_location) _jump)) (Math|Vector|MakeVector 0.0 0.0 (+ (.z _relative_location) _jump)) (Math|Trig|Sin(Radians) (* (Variables|Default|GetNewVar_0) 1e+01))) (Math|Rotator|MakeRotator (.roll (Math|Rotator|Lerp(Rotator) (Math|Rotator|MakeRotator (* _balencement -1.0) 0.0 0.0) (Math|Rotator|MakeRotator _balencement 0.0 0.0) (Math|Trig|Sin(Radians) (* (Variables|Default|GetNewVar_0) 5.0)))) 0.0 0.0) false false))

(fn ConstructionScript)