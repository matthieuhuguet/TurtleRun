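; Vehicle prop Blueprint that fakes driving motion through wheel spin and body bobbing.
; BeginPlay caches the Veicule component's relative location and rotation.
; Each Tick spins the four wheels by TaxiSpeed, without scaling by delta time.
; Accumulated time drives sine-based lerps that bounce the body vertically by Jump and rock its roll by Balencement at half that frequency.
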(event EventBeginPlay
  (bind _veicule (Variables|Default|GetVeicule))
  ;[0.5422 0.386 1] Position meshes
  (Variables|TA|SetRelative%20Location (Variables|/Script/Engine.SceneComponent|GetRelativeLocation _veicule))
  (Variables|TA|SetRelative%20Rotation (Variables|/Script/Engine.SceneComponent|GetRelativeRotation _veicule)))

(event Collision|EventActorBeginOverlap
  (params (OtherActor :type Actor%20Object%20Reference)))

(event EventTick
  (params (DeltaSeconds :type Float%20%28single-precision%29))
  (bind _jump (Variables|TA|Getjump))
  (bind _balencement (Variables|TA|Getbalencement))
  (bind _relative_location (Variables|TA|GetRelative%20Location))
  ;[1 0.3444 0.8431] Valeure de repetition
  (Variables|TA|Setvariable_on%20sais%20pas%20trop%20tkt (+ DeltaSeconds (Variables|TA|Getvariable_on%20sais%20pas%20trop%20tkt)))
  ;[0.09375 0.6472 1] Rotation des roues
  (Transformation|AddLocalRotation (Variables|Default|GetRoue_1) (Math|Rotator|MakeRotator 0.0 (Variables|TA|GetTaxiSpeed) 0.0) false false)
  (Transformation|SetRelativeLocationAndRotation (Variables|Default|GetVeicule) (Math|Vector|Lerp(Vector) (Math|Vector|MakeVector 0.0 0.0 (- (.z _relative_location) _jump)) (Math|Vector|MakeVector 0.0 0.0 (+ (.z _relative_location) _jump)) (Math|Trig|Sin(Radians) (* (Variables|TA|Getvariable_on%20sais%20pas%20trop%20tkt) 1e+01))) (Math|Rotator|MakeRotator (.roll (Math|Rotator|Lerp(Rotator) (Math|Rotator|MakeRotator (* _balencement -1.0) 0.0 0.0) (Math|Rotator|MakeRotator _balencement 0.0 0.0) (Math|Trig|Sin(Radians) (* (Variables|TA|Getvariable_on%20sais%20pas%20trop%20tkt) 5.0)))) 0.0 0.0) false false))

(fn ConstructionScript)