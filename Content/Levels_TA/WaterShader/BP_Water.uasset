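; BP_Water is a water actor that bobs its PlaneWater component up and down.
; BeginPlay stores the plane's starting relative location as the reference height.
; Tick accumulates time and feeds a slowed sine into a vector Lerp between heights offset by Hauteur below and above that start.
; The sine is not remapped to 0–1, so the motion dips further below the start than it rises.
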(event EventBeginPlay
  (Variables|Default|SetRelative%20Location (Variables|/Script/Engine.SceneComponent|GetRelativeLocation (Variables|Default|GetPlaneWater))))

(event Collision|EventActorBeginOverlap
  (params (OtherActor :type Actor%20Object%20Reference)))

(event EventTick
  (params (DeltaSeconds :type Float%20%28single-precision%29))
  (bind _relative_location (Variables|Default|GetRelative%20Location))
  (bind _hauteur (Variables|Default|Gethauteur))
  (Variables|Default|SetNewVar_0 (+ DeltaSeconds (Variables|Default|GetNewVar_0)))
  (Transformation|SetRelativeLocation (Variables|Default|GetPlaneWater) (Math|Vector|Lerp(Vector) (Math|Vector|MakeVector 0.0 0.0 (- (.z _relative_location) _hauteur)) (Math|Vector|MakeVector 0.0 0.0 (+ (.z _relative_location) _hauteur)) (Math|Trig|Sin(Radians) (* (Variables|Default|GetNewVar_0) 0.5))) false false))

(fn ConstructionScript)